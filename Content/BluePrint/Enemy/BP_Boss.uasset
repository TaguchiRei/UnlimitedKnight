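; BP_Boss is an enemy boss character that chases the player and switches to attacking at close range.
; Each tick it turns on yaw only to face player 0, with a 90-degree offset.
; Beyond MoveLimit it moves straight toward the player horizontally through forced CharacterMovement input scaled by Speed, without pathfinding.
; It sets the Attacking flag on ABP_Boss, true within range and false while chasing.
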(event EventBeginPlay)

(event Collision|EventActorBeginOverlap
  (params (OtherActor :type Actor%20Object%20Reference)))

(event EventTick
  (params (DeltaSeconds :type Float%20%28single-precision%29))
  (bind _returnvalue (Transformation|GetActorLocation))
  (bind _returnvalue_2 (Game|GetPlayerCharacter 0))
  (bind _returnvalue_3 (Transformation|GetActorLocation _returnvalue_2))
  (bind _returnvalue_4 (- _returnvalue_3 _returnvalue))
  (bind (_x _y) (Math|Vector|BreakVector _returnvalue_4))
  (Transformation|SetActorRotation (Math|Rotator|MakeRotator 0.0 0.0 (- (.Yaw (Math|Rotator|BreakRotator (Math|Rotator|FindLookatRotation (Transformation|GetActorLocation) (Transformation|GetActorLocation (Game|GetPlayerCharacter 0))))) 9e+01)))
  (bind _asabp_boss (Utilities|Casting|CastToABP_Boss (Components|SkeletalMesh|GetAnimInstance (Variables|Character|GetMesh))))
  (if (> (Math|Vector|VectorLength _returnvalue_4) (Variables|Default|GetMoveLimit))
    (Variables|/Game/BluePrint/Enemy/ABP_Boss.ABP_Boss_C|SetAttacking _asabp_boss false)
    (Class|PawnMovementComponent|AddInputVector (Variables|Character|GetCharacterMovement) (* (Math|Vector|Normalize (Math|Vector|MakeVector _x _y 0.0)) (Variables|Default|GetSpeed)) true)
    (else
      (Variables|/Game/BluePrint/Enemy/ABP_Boss.ABP_Boss_C|SetAttacking _asabp_boss true))))

(fn ConstructionScript)