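; Boss enemy actor that steers toward player controller 0's actor location every frame.
; Tick builds a horizontal velocity from the direction to that location, capped by Speed and scaled by delta time, and sets it as the Cone component's physics linear velocity, with Z zeroed.
; It also rotates the actor to face that velocity and prints the vector to screen for debugging.
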(event EventBeginPlay)

(event Collision|EventActorBeginOverlap
  (params (OtherActor :type Actor%20Object%20Reference)))

(event EventTick
  (params (DeltaSeconds :type Float%20%28single-precision%29))
  (bind _returnvalue (Game|GetPlayerController 0))
  (bind _returnvalue_2 (Transformation|GetActorLocation))
  (bind _speed (Variables|Default|GetSpeed))
  (bind _speed_2 (Variables|Default|GetSpeed))
  (bind _returnvalue_3 (Transformation|GetActorLocation _returnvalue))
  (bind _returnvalue_4 (- _returnvalue_3 _returnvalue_2))
  (bind _returnvalue_5 (Math|Vector|Normalize _returnvalue_4))
  (bind _returnvalue_6 (* _returnvalue_4 _speed))
  (bind _returnvalue_7 (Math|Vector|VectorLength _returnvalue_6))
  (bind _returnvalue_8 (Math|Float|Clamp(Float) _returnvalue_7 0.0 _speed_2))
  (bind _returnvalue_9 (* _returnvalue_5 _returnvalue_8))
  (bind _returnvalue_10 (* _returnvalue_9 DeltaSeconds))
  (bind (_x _y) (Math|Vector|BreakVector _returnvalue_10))
  (bind _returnvalue_11 (Math|Vector|MakeVector _x _y 0.0))
  (Physics|SetPhysicsLinearVelocity (Variables|Default|GetCone) _returnvalue_11 false "None")
  (Transformation|SetActorRotation (Math|Conversions|RotationFromXVector (Math|Vector|Normalize _returnvalue_11)))
  (Development|PrintString (Utilities|String|ToString(Vector) _returnvalue_11)))

(fn ConstructionScript)